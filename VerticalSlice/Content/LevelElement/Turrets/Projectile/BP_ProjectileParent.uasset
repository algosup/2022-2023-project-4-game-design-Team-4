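; Base projectile for turrets, which damages enemies on impact.
; On BeginPlay it copies its gravity, initial speed and max speed variables into the ProjectileMovement component.
; When the hit sphere collides, it applies damage only to BP_Enemy_Parent actors, then spawns a Niagara hit effect and destroys itself whatever it struck.
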(event OnComponentHit(SphereHit)
  (params (HitComponent :type Primitive%20Component%20Object%20Reference) (OtherActor :type Actor%20Object%20Reference) (OtherComp :type Primitive%20Component%20Object%20Reference) (NormalImpulse :type Vector :default "0, 0, 0") (Hit :type Hit%20Result%20Structure%20%28by%20ref%29))
  ;[1 1 1] damage
  (Utilities|FlowControl|Sequence
    (:then_0
      (bind _asbp_enemy_parent (Utilities|Casting|CastToBP_Enemy_Parent OtherActor))
      (Game|Damage|ApplyDamage _asbp_enemy_parent (Variables|Default|GetDamageProjectile) 0 0))
    (:then_1
      (Niagara|SpawnSystematLocation "/Game/LevelElement/Turrets/Projectile/NSHitEnemies.NSHitEnemies" (Transformation|GetActorLocation))
      (Actor|DestroyActor))))

(event EventBeginPlay
  (bind _projectilemovement (Variables|Default|GetProjectileMovement))
  ;[1 1 1] Speed projectile
  (Variables|/Script/Engine.ProjectileMovementComponent|SetProjectileGravityScale _projectilemovement (Variables|Default|GetProjectileGravity))
  (Variables|/Script/Engine.ProjectileMovementComponent|SetInitialSpeed _projectilemovement (Variables|Default|GetProjectileInitialSpeed))
  (Variables|/Script/Engine.ProjectileMovementComponent|SetMaxSpeed _projectilemovement (Variables|Default|GetProjectileMaxSpeed)))

(event Collision|EventActorBeginOverlap
  (params (OtherActor :type Actor%20Object%20Reference)))

(event EventTick
  (params (DeltaSeconds :type Float%20%28single-precision%29))
  ;[1 1 1] damage
)

(fn ConstructionScript)