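; Tower defense game mode that runs enemy waves and enables mouse cursor, click and hover input.
; Each wave's counts per mutant type load from a data table row named by wave number into a class-to-count map.
; A looping timer sends a randomly picked remaining type to a random SpawnPoint, advancing the wave once none remain and the Enemies list is empty.
; An event hides turret-selection widgets on all slots.
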(event Custom|ActivateSpawner
  (bind _listofspawnpoint (Variables|Default|GetListOfSpawnPoint))
  (if (> (Variables|Default|GetNumberOfEnemies) 0)
    (bind _enemychosen (CallFunction|ChooseEnemy))
    (Default|SpawnEnemy (Utilities|Array|Get(acopy) _listofspawnpoint (Math|Random|RandomIntegerinRange 0 (- (Utilities|Array|Length _listofspawnpoint) 1))) _enemychosen)
    (else
      (bind _returnvalue (CallFunction|IsLevelEnd))
      (if _returnvalue
        (CallFunction|OnLevelEnd)))))

(event Custom|OnLevelEnd
  (bind _result (Math|Integer|IncrementInt (Variables|Default|GetWaveNumber))
    (:%20%20
      (CallFunction|SetNumberEnemiesPerWave _result))))

(event Custom|HiddenWBTurretSelect
  (bind _outactors (Actor|GetAllActorsOfClass "/Game/LevelElement/Turrets/BP_Slot.BP_Slot_C"))
  (for (_ _array_index) _outactors
    (Rendering|SetVisibility (Variables|/Game/LevelElement/Turrets/BP_Slot.BP_Slot_C|GetWidget (Utilities|Array|Get(acopy) _outactors _array_index)) false false)))

(event EventBeginPlay
  (bind _returnvalue (Game|GetPlayerController 0))
  (Utilities|FlowControl|Sequence
    (:then_0
      (bind _outactors (Actor|GetAllActorsOfClass "/Game/LevelElement/GoalAndSpawn/SpawnPoint.SpawnPoint_C"))
      (Variables|Default|SetListOfSpawnPoint _outactors)
      ;[1 1 1] TImer between 2 enemies
      (Utilities|Time|SetTimerbyEvent (delegate Custom|ActivateSpawner) 4.0 true)
      (CallFunction|SetNumberEnemiesPerWave (Variables|Default|GetWaveNumber)))
    (:then_1
      (Variables|/Script/Engine.PlayerController|SetbShowMouseCursor _returnvalue true)
      (Variables|/Script/Engine.PlayerController|SetbEnableClickEvents _returnvalue true)
      (Variables|/Script/Engine.PlayerController|SetbEnableMouseOverEvents _returnvalue true))))

(fn ConstructionScript)

(fn SetNumberEnemiesPerWave
  (params (WaveNumber :type Integer))
  (bind _returnvalue (Utilities|GetDataTableRow "/Game/Enemies/WaveDetailsDataTable.WaveDetailsDataTable" (Utilities|String|StringToName (Utilities|String|ToString(Integer) WaveNumber)))
    (:then
      (bind _output_get (Variables|Default|SetEnemyList (Utilities|Map|MakeMap "/Game/Enemies/BP_Mutant_Small.BP_Mutant_Small_C" (.mutant_small _returnvalue) "/Game/Enemies/BP_Mutant_Large.BP_Mutant_Large_C" (.mutant_large _returnvalue) "/Game/Enemies/BP_Mutant_XL.BP_Mutant_XL_C" (.mutant_xl _returnvalue))))
      (Variables|Default|SetNumberOfEnemies 0)
      (bind _values (Utilities|Map|Values _output_get))
      (for _array_element _values
        (Variables|Default|SetNumberOfEnemies (+ _array_element (Variables|Default|GetNumberOfEnemies)))))))

(fn ChooseEnemy
  (bind _keys (Utilities|Map|Keys (Variables|Default|GetEnemyList) :!label _label))
  (bind _output_get (Variables|Default|SetChosenEnemy (Utilities|Array|Get(acopy) _keys (Math|Random|RandomInteger (Utilities|Array|Length _keys)))))
  (Variables|Default|SetEnemyNumber (.Value (Utilities|Map|Find (Variables|Default|GetEnemyList) _output_get)))
  (if (> (.Value (Utilities|Map|Find (Variables|Default|GetEnemyList) _output_get)) 0)
    (Utilities|Map|Add (Variables|Default|GetEnemyList) (Variables|Default|GetChosenEnemy) (- (Variables|Default|GetEnemyNumber) 1))
    (Variables|Default|SetNumberOfEnemies (- (Variables|Default|GetNumberOfEnemies) 1))
    (return (Variables|Default|GetChosenEnemy))
    (else
      (goto _label))))

(fn IncreaseNumberWave
  (bind _result (Math|Integer|IncrementInt (Variables|Default|GetWaveNumber))
    (:%20%20
      (CallFunction|SetNumberEnemiesPerWave _result))))

(fn IsLevelEnd
  (return (<= (Utilities|Array|Length (Variables|Default|GetEnemies)) 0)))