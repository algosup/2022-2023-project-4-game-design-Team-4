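; Player controller for the tower defense game that holds the player's resource count and handles the end of the game.
; On BeginPlay it sets Game and UI input mode with the mouse locked to the viewport and the cursor visible during capture.
; AddResources increments the resource total.
; End shows the end-game widget, hides the mouse cursor and pauses the game.
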(event Custom|Add%20Resources
  (params (MoreRessources :type Integer))
  (Variables|Default|SetRessources (+ (Variables|Default|GetRessources) MoreRessources)))

(event Custom|End
  (bind _returnvalue (UserInterface|CreateWidget "/Game/HUD/EndGameWidget.EndGameWidget_C"))
  (UserInterface|Viewport|AddtoViewport _returnvalue 0)
  (Variables|Default|SetbShowMouseCursor false)
  (Game|SetGamePaused true))

(event EventBeginPlay
  (Input|SetInputModeGameandUI self 0 "LockAlways" false))

(fn ConstructionScript)