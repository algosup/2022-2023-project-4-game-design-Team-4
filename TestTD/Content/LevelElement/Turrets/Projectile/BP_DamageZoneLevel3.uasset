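; BP_DamageZoneLevel3 is a short-lived turret area-damage actor that spawns a ZoneDamage effect after a brief delay and destroys itself seconds later.
; Its Sphere overlap subtracts a fixed amount of HP from each BP_Enemy_Parent as it begins overlapping.
; At zero HP, it hides the health bar, stops movement and collision, and plays a random death animation.
; Delayed enemy destruction runs on this actor, using one stored enemy reference.
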(event OnComponentBeginOverlap(Sphere)
  (params (OverlappedComponent :type Primitive%20Component%20Object%20Reference) (OtherActor :type Actor%20Object%20Reference) (OtherComp :type Primitive%20Component%20Object%20Reference) (OtherBodyIndex :type Integer) (bFromSweep :type Boolean) (SweepResult :type Hit%20Result%20Structure%20%28by%20ref%29))
  (bind _asbp_enemy_parent (Utilities|Casting|CastToBP_Enemy_Parent OtherActor))
  (Variables|Default|SetAs%20BP%20Enemy%20Parent _asbp_enemy_parent)
  (bind _output_get (Variables|/Game/Enemies/BP_Enemy_Parent.BP_Enemy_Parent_C|SetHP _asbp_enemy_parent (- (Variables|/Game/Enemies/BP_Enemy_Parent.BP_Enemy_Parent_C|GetHP _asbp_enemy_parent) 4e+02)))
  (if (<= _output_get 0.0)
    (Rendering|SetVisibility (Variables|/Game/Enemies/BP_Enemy_Parent.BP_Enemy_Parent_C|GetBP_HPEnemy (Variables|Default|GetAs%20BP%20Enemy%20Parent)) false false)
    (Variables|/Script/Engine.CharacterMovementComponent|SetMaxWalkSpeed (Variables|/Script/Engine.Character|GetCharacterMovement (Variables|Default|GetAs%20BP%20Enemy%20Parent)) 0.0)
    (Variables|/Game/Enemies/BP_Enemy_Parent.BP_Enemy_Parent_C|SetHPGood (Variables|Default|GetAs%20BP%20Enemy%20Parent) false)
    (Collision|SetCollisionEnabled (Variables|/Script/Engine.Character|GetCapsuleComponent (Variables|Default|GetAs%20BP%20Enemy%20Parent)) "NoCollision")
    (Components|Animation|PlayAnimation (Variables|/Script/Engine.Character|GetMesh (Variables|Default|GetAs%20BP%20Enemy%20Parent)) (Utilities|Select :Index (Math|Random|RandomIntegerinRange 0 3) :Option%200 (Variables|/Game/Enemies/BP_Enemy_Parent.BP_Enemy_Parent_C|GetDeath1 (Variables|Default|GetAs%20BP%20Enemy%20Parent)) :Option%201 (Variables|/Game/Enemies/BP_Enemy_Parent.BP_Enemy_Parent_C|GetDeath2 (Variables|Default|GetAs%20BP%20Enemy%20Parent)) :Option%202 (Variables|/Game/Enemies/BP_Enemy_Parent.BP_Enemy_Parent_C|GetDeath3 (Variables|Default|GetAs%20BP%20Enemy%20Parent)) :Option%203 (Variables|/Game/Enemies/BP_Enemy_Parent.BP_Enemy_Parent_C|GetDeath4 (Variables|Default|GetAs%20BP%20Enemy%20Parent))) false)
    (Utilities|FlowControl|Delay 2.2)
    (Actor|DestroyActor (Variables|Default|GetAs%20BP%20Enemy%20Parent))))

(event EventBeginPlay
  (Utilities|FlowControl|Delay 0.2)
  (Niagara|SpawnSystematLocation "/Game/LevelElement/Turrets/Projectile/ZoneDamage.ZoneDamage" (Transformation|GetActorLocation))
  (Utilities|FlowControl|Delay 3.0)
  (Actor|DestroyActor))

(event Collision|EventActorBeginOverlap
  (params (OtherActor :type Actor%20Object%20Reference)))

(event EventTick
  (params (DeltaSeconds :type Float%20%28single-precision%29)))

(fn ConstructionScript)