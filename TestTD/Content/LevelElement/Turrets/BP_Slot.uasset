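; BP_Slot is a clickable turret slot in the level that opens the turret selection menu.
; Mouse hover, click and release events on the Slot component swap its material for visual feedback.
; When CanSpawnATurret is true, a click removes existing WBP_TurretSelect widgets and shows a new one; otherwise it applies the disabled material.
; The assignment passing this slot to the widget as EmptySlot is unconnected and never runs.
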(event OnBeginCursorOver(Slot)
  (params (TouchedComponent :type Primitive%20Component%20Object%20Reference))
  (Rendering|Material|SetMaterial (Variables|Default|GetSlot) 0 "/Game/LevelElement/Turrets/Material/M_Turret_MouseOver.M_Turret_MouseOver"))

(event OnEndCursorOver(Slot)
  (params (TouchedComponent :type Primitive%20Component%20Object%20Reference))
  (Rendering|Material|SetMaterial (Variables|Default|GetSlot) 0 "/Game/LevelElement/Turrets/Material/M_Turret_MouseOut.M_Turret_MouseOut"))

(event OnClicked(Slot)
  (params (TouchedComponent :type Primitive%20Component%20Object%20Reference) (ButtonPressed :type Key%20Structure :default "None"))
  (if (Variables|Default|GetcanSpawnATurret)
    (Rendering|Material|SetMaterial (Variables|Default|GetSlot) 0 "/Game/LevelElement/Turrets/Material/M_Turret_MouseClick.M_Turret_MouseClick")
    (bind _foundwidgets (Widget|GetAllWidgetsOfClass "/Game/HUD/WBP_TurretSelect.WBP_TurretSelect_C" false))
    (for _array_element _foundwidgets
      (Widget|RemovefromParent _array_element))
    (bind _returnvalue (UserInterface|CreateWidget "/Game/HUD/WBP_TurretSelect.WBP_TurretSelect_C"))
    (UserInterface|Viewport|AddtoViewport _returnvalue 0)
    (else
      (Rendering|Material|SetMaterial (Variables|Default|GetSlot) 0 "/Game/LevelElement/Turrets/Material/M_Turret_MouseDisabled.M_Turret_MouseDisabled"))))

(event OnReleased(Slot)
  (params (TouchedComponent :type Primitive%20Component%20Object%20Reference) (ButtonReleased :type Key%20Structure :default "None"))
  (Rendering|Material|SetMaterial (Variables|Default|GetSlot) 0 "/Game/LevelElement/Turrets/Material/M_Turret_MouseOver.M_Turret_MouseOver"))

(event EventBeginPlay)

(event Collision|EventActorBeginOverlap
  (params (OtherActor :type Actor%20Object%20Reference)))

(event EventTick
  (params (DeltaSeconds :type Float%20%28single-precision%29)))

(fn ConstructionScript)