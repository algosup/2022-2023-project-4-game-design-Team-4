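; Parent enemy for a tower defense game that walks via AI MoveTo to the first GoalOfEnemies actor, retrying on failure and destroying itself on arrival.
; Damage drains HP until death, which stops movement, hides the HP display, disables capsule collision and plays a random death animation.
; After a delay it is destroyed, removed from the GameMode's enemy list and grants player resources.
; SetLife scales health by wave.
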(event Custom|GoToGoal
  (if (Variables|Default|GetHPGood)
    (Utilities|FlowControl|Delay 0.2)
    (Variables|/Script/Engine.CharacterMovementComponent|SetMaxWalkSpeed (Variables|Character|GetCharacterMovement) (Variables|Default|GetSpeedMove))
    (bind _outactors (Actor|GetAllActorsOfClass "/Game/LevelElement/GoalAndSpawn/GoalOfEnemies.GoalOfEnemies_C"))
    (AI|AIMoveTo self "0, 0, 0" (Utilities|Array|Get(acopy) _outactors) 2e+02 false
      (:OnSuccess
        (Actor|DestroyActor))
      (:OnFail
        (CallFunction|GotoGoal)))))

(event EventBeginPlay
  (CallFunction|GotoGoal))

(event Game|Damage|EventAnyDamage
  (params (Damage :type Float%20%28single-precision%29) (DamageType :type Damage%20Type%20Object%20Reference) (InstigatedBy :type Controller%20Object%20Reference) (DamageCauser :type Actor%20Object%20Reference))
  (Variables|Default|SetHP (- (Variables|Default|GetHP) Damage))
  (if (<= (Variables|Default|GetHP) 0.0)
    (Rendering|SetVisibility (Variables|Default|GetBP_HPEnemy) false false)
    (Variables|/Script/Engine.CharacterMovementComponent|SetMaxWalkSpeed (Variables|Character|GetCharacterMovement) 0.0)
    (Variables|Default|SetHPGood false)
    (Collision|SetCollisionEnabled (Variables|Collision|GetCapsuleComponent) "NoCollision")
    (Components|Animation|PlayAnimation (Variables|Character|GetMesh) (Utilities|Select :Index (Math|Random|RandomIntegerinRange 0 3) :Option%200 (Variables|Default|GetDeath1) :Option%201 (Variables|Default|GetDeath2) :Option%202 (Variables|Default|GetDeath3) :Option%203 (Variables|Default|GetDeath4)) false)
    (Utilities|FlowControl|Delay 3.0)
    (Actor|DestroyActor)
    (bind _asgm_tower_defense (Utilities|Casting|CastToGM_TowerDefense (Game|GetGameMode)))
    (Utilities|Array|RemoveItem (Variables|/Game/TD_Blueprints/GM_TowerDefense.GM_TowerDefense_C|GetEnemies _asgm_tower_defense) self)
    (bind _aspc_tower_defense (Utilities|Casting|CastToPC_TowerDefense (Game|GetPlayerController 0)))
    (Default|AddResources _aspc_tower_defense)))

(fn ConstructionScript)

(fn AddLife
  (params (Wave :type Integer) (Percent :type Float%20%28single-precision%29))
  (Variables|Default|SetHpMax (* (Variables|Default|GetHP) (+ Percent 1.0))))

(fn SetLife
  (params (Wave :type Integer) (Percent :type Float%20%28single-precision%29))
  (bind _output_get (Variables|Default|SetHpMax (* (+ 1.0 (* (Math|Conversions|ToFloat(Integer) Wave) Percent)) (Variables|Default|GetHP))))
  (Variables|Default|SetHP _output_get))