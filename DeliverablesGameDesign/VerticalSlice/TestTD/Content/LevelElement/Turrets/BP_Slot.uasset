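; BP_Slot is a clickable empty turret slot for the tower defense mode, with a widget component holding the turret selection menu.
; At BeginPlay it passes itself to WBP_TurretSelect and caches GM_TowerDefense.
; Cursor events swap the slot material as feedback.
; Clicking calls the GameMode's HiddenWBTurretSelect, then toggles the menu, which auto-hides after a short delay once shown.
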(event OnBeginCursorOver(Slot)
  (params (TouchedComponent :type Primitive%20Component%20Object%20Reference))
  (Rendering|Material|SetMaterial (Variables|Default|GetSlot) 0 "/Game/LevelElement/Turrets/Material/M_Turret_MouseOver.M_Turret_MouseOver"))

(event OnEndCursorOver(Slot)
  (params (TouchedComponent :type Primitive%20Component%20Object%20Reference))
  (Rendering|Material|SetMaterial (Variables|Default|GetSlot) 0 "/Game/LevelElement/Turrets/Material/M_Turret_MouseOut.M_Turret_MouseOut"))

(event OnClicked(Slot)
  (params (TouchedComponent :type Primitive%20Component%20Object%20Reference) (ButtonPressed :type Key%20Structure :default "None"))
  (bind _widget (Variables|Default|GetWidget))
  (Default|HiddenWBTurretSelect (Variables|Default|GetGM))
  (Rendering|Material|SetMaterial (Variables|Default|GetSlot) 0 "/Game/LevelElement/Turrets/Material/M_Turret_MouseClick.M_Turret_MouseClick")
  (if (Rendering|IsVisible (Variables|Default|GetWidget))
    _
    (else
      (Rendering|SetVisibility _widget true false)
      (Utilities|FlowControl|Delay 3.0)))
  (Rendering|SetVisibility _widget false false))

(event OnReleased(Slot)
  (params (TouchedComponent :type Primitive%20Component%20Object%20Reference) (ButtonReleased :type Key%20Structure :default "None"))
  (Rendering|Material|SetMaterial (Variables|Default|GetSlot) 0 "/Game/LevelElement/Turrets/Material/M_Turret_MouseOver.M_Turret_MouseOver"))

(event EventBeginPlay
  (bind _aswbp_turret_select (Utilities|Casting|CastToWBP_TurretSelect (UserInterface|GetUserWidgetObject (Variables|Default|GetWidget))))
  (Variables|/Game/HUD/WBP_TurretSelect.WBP_TurretSelect_C|SetEmptySlot _aswbp_turret_select self)
  (bind _asgm_tower_defense (Utilities|Casting|CastToGM_TowerDefense (Game|GetGameMode)))
  (Variables|Default|SetGM _asgm_tower_defense))

(fn ConstructionScript)